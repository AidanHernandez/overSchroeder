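; BP_meatier_warning is a ground warning marker that telegraphs a falling BP_meatier.
; BeginPlay stores the timer and pins the actor to a fixed height.
; Tick spins it by a per-frame yaw step and shrinks it from unit scale (StartingScale is unused), then spawns BP_meatier high overhead and destroys itself when time expires.
; An unconnected chain would stun the lobby player controller but never runs.
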(event `self.ReceiveBeginPlay`
  (bind _returnvalue (`self.GetTransform`))
  ;[1 1 1] Start starting values
  (set `self.timer` (`self.timer start`))
  (set `self.starting scale` (.x (.scale _returnvalue)))
  (`self.K2_SetActorTransform` (`KismetMathLibrary.MakeTransform` (`KismetMathLibrary.MakeVector` (.x (.location _returnvalue)) (.y (.location _returnvalue)) -49.0))))

(event `self.ReceiveTick`
  (params (DeltaSeconds :type "Float (single-precision)"))
  (bind _returnvalue (`self.GetTransform`))
  (bind _returnvalue_2 (`self.GetTransform`))
  ;[1 1 1] Shrink warning until it dissapears
  (bind _output_get (set `self.timer` (- (`self.timer`) DeltaSeconds)))
  (bind _returnvalue_3 (`KismetMathLibrary.Lerp` 0.0 1.0 (`KismetMathLibrary.SafeDivide` _output_get (`self.timer start`))))
  (`self.K2_SetActorTransform` (`KismetMathLibrary.MakeTransform` (.location _returnvalue_2) (`KismetMathLibrary.MakeRotator` 0.0 0.0 (+ (.yaw (.rotation _returnvalue_2)) 3.0)) (`KismetMathLibrary.MakeVector` _returnvalue_3 _returnvalue_3 _returnvalue_3)))
  (if (<= (`self.timer`) 0.0)
    (`|SpawnActorFromClass` "/Game/blueprints/BP_meatier.BP_meatier_C" (`KismetMathLibrary.MakeTransform` (`KismetMathLibrary.MakeVector` (.x (.location _returnvalue)) (.y (.location _returnvalue)) (+ (.z (.location _returnvalue)) 1500.0))) "Undefined" "MultiplyWithRoot" null null)
    (`self.K2_DestroyActor`)))

(fn `UserConstructionScript`)