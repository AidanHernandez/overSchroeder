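; Stove appliance Blueprint that holds a single cookware item, either a Pot or a Pan.
; AddApplianc places the selected item when the stove is empty, showing Cube1 with a material specific to that item.
; When occupied, an empty selection removes the item, hides the cube and returns the item's name, while any other selection fails.
; Event graph and construction script are empty.
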(fn `addApplianc`
  (params (Selection :type String))
  (returns (worked :type Boolean) (itemOnStove :type String))
  (bind _cube1 (`self.Cube1`))
  (if (`self.applianceAdded`)
    (if (`KismetStringLibrary.EqualEqual_StrStr` Selection)
      (`SceneComponent.SetHiddenInGame` (`self.Cube1`) true false)
      (set `self.applianceAdded` false)
      (set `self.itemOnStovetemp` (`self.itemOnStove`))
      (set `self.itemOnStove` "")
      (return true (`self.itemOnStovetemp`))
      (else
        (return false "")))
    (else
      (switch `string` Selection
        (:`Pot`
          (`SceneComponent.SetHiddenInGame` _cube1 false false)
          (`PrimitiveComponent.SetMaterial` _cube1 0 "/Engine/MapTemplates/Materials/BasicAsset01.BasicAsset01")
          (set `self.itemOnStove` "Pot"))
        (:`Pan`
          (`SceneComponent.SetHiddenInGame` _cube1 false false)
          (`PrimitiveComponent.SetMaterial` _cube1 0 "/Engine/EngineDebugMaterials/BoneWeightMaterial.BoneWeightMaterial")
          (set `self.itemOnStove` "Pan")))
      (set `self.applianceAdded` true)
      (return true (`self.itemOnStove`)))))

(fn `UserConstructionScript`)