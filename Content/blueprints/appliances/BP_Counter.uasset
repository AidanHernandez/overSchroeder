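; BP_Counter is a counter appliance that holds one item at a time, placed or taken through AddAppliance.
; On an empty counter, a Pot, Pan or Horse selection stores the name and reveals a single StaticMesh, distinguished only by material swap.
; On an occupied counter, an empty selection hides the mesh and returns the stored item, while any other selection fails.
; The event graph and construction script are empty.
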(fn `addAppliance`
  (params (Selection :type String))
  (returns (worked :type Boolean) (itemOnStove :type String))
  (bind _staticmesh (`self.StaticMesh`))
  (if (`self.itemAdded`)
    (if (`KismetStringLibrary.EqualEqual_StrStr` Selection)
      (`SceneComponent.SetHiddenInGame` (`self.StaticMesh`) true false)
      (set `self.itemAdded` false)
      (set `self.itemOnCountertemp` (`self.itemOnCounter`))
      (set `self.itemOnCounter` "")
      (return true (`self.itemOnCountertemp`))
      (else
        (return false "")))
    (else
      (switch `string` Selection
        (:`Pot`
          (`PrimitiveComponent.SetMaterial` _staticmesh 0 "/Engine/MapTemplates/Materials/BasicAsset01.BasicAsset01")
          (set `self.itemOnCounter` "Pot"))
        (:`Pan`
          (`PrimitiveComponent.SetMaterial` _staticmesh 0 "/Engine/EngineDebugMaterials/BoneWeightMaterial.BoneWeightMaterial")
          (set `self.itemOnCounter` "Pan"))
        (:`horse`
          (`PrimitiveComponent.SetMaterial` _staticmesh 0 "/Engine/EditorMaterials/Cascade/CASC_ModuleDisable_MAT.CASC_ModuleDisable_MAT")
          (set `self.itemOnCounter` "Horse")))
      (set `self.itemAdded` true)
      (`SceneComponent.SetHiddenInGame` (`self.StaticMesh`) false false)
      (return true (`self.itemOnCounter`)))))

(fn `UserConstructionScript`)