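; Deep fryer appliance that takes an item, cooks it on a timer and hands it back to the player.
; FryerActivated shows the item in the basket and sets its cook time, with Horse the only item type handled.
; CookingStarts toggles the basket's height through a FlipFlop-driven timeline and starts a W_CookTime widget timer.
; When BasketMove receives timer completion, it clears the widget, toggles the basket and passes the cooked result to BP_TopDownCharacter.
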(event `self.ReceiveBeginPlay`
  (set `self.intialLocation` (`SceneComponent.RelativeLocation` (`self.basket`))))

(event `basketMove`
  (params (timerDone :type Boolean))
  (bind (_intiallocation_x _intiallocation_y _intiallocation_z) (`KismetMathLibrary.BreakVector` (`self.intialLocation`)))
  (if timerDone
    (set `/Game/widgets/W_CookTime.timerDone` true (`self.cookTimeW`))
    (`WidgetComponent.SetWidget` (`self.cookTimeWidget`) null)
    (set `self.cookingStarted` false)
    (set `self.Cooked?` (`/Game/widgets/W_CookTime.cooked?` (`self.cookTimeW`)))
    (`self.returnItem`))
  (`/Engine/EditorBlueprintResources/StandardMacros.FlipFlop`
    (:`A`
      (set `self.basketDown` false)
      (bind (_direction _newtrack_0) (`Timeline|Timeline` :!via `PlayFromStart` :!label _label)
        (:`Update`
          (`SceneComponent.K2_SetRelativeLocation` (`self.basket`) (`KismetMathLibrary.VLerp` (`KismetMathLibrary.MakeVector` _intiallocation_x _intiallocation_y _intiallocation_z) (`KismetMathLibrary.MakeVector` _intiallocation_x _intiallocation_y -100.0) _newtrack_0) false false)
          (`KismetSystemLibrary.Delay` _newtrack_0)
          (set `self.currentlyMoving` false))))
    (:`B`
      (set `self.basketDown` true)
      (goto _label :!via `ReverseFromEnd`))))

(event `returnItem`
  (switch `string` (`self.iteminHand`)
    (:`Horse`
      (`SceneComponent.SetHiddenInGame` (`self.StaticMesh1`) true false)
      (bind _asbp_top_down_character (cast `/Game/TopDown/Blueprints/BP_TopDownCharacter` (`GameplayStatics.GetPlayerCharacter` 0)))
      (bind _cube (`/Game/TopDown/Blueprints/BP_TopDownCharacter.Cube` _asbp_top_down_character))
      (`SceneComponent.SetHiddenInGame` _cube false false)
      (`PrimitiveComponent.SetMaterial` _cube 0 "/Engine/EditorMaterials/Cascade/CASC_ModuleDisable_MAT.CASC_ModuleDisable_MAT")
      (set `/Game/TopDown/Blueprints/BP_TopDownCharacter.itemInHandsCooked` (`self.Cooked?`) _asbp_top_down_character))))

(fn `cookingStarts`
  (set `self.currentlyMoving` true)
  (`self.basketMove` false)
  (bind _returnvalue (`|CreateWidget` "/Game/widgets/W_CookTime.W_CookTime_C"))
  (set `self.cookTimeW` _returnvalue)
  (`WidgetComponent.SetWidget` (`self.cookTimeWidget`) _returnvalue)
  (set `/Game/widgets/W_CookTime.cookTIme` (`self.cookTime`) _returnvalue)
  (`/Game/widgets/W_CookTime.startTimer` _returnvalue self)
  (set `self.cookingStarted` true))

(fn `fryerActivated`
  (params (NewParam :type String))
  (returns (NewParam1 :type String) (`added?` :type Boolean))
  (bind _staticmesh1 (`self.StaticMesh1`))
  (set `self.iteminHand` NewParam)
  (if (not (`self.currentlyMoving`))
    (switch `string` NewParam
      (:`Horse`
        (`SceneComponent.SetHiddenInGame` _staticmesh1 false false)
        (`PrimitiveComponent.SetMaterial` _staticmesh1 0 "/Engine/EditorMaterials/Cascade/CASC_ModuleDisable_MAT.CASC_ModuleDisable_MAT")
        (set `self.cookTime` 5.0)
        (return "" true)))))

(fn `UserConstructionScript`)