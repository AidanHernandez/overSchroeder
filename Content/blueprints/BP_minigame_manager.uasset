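; Minigame manager that picks a random entry from Games on BeginPlay and again six seconds after each recognized pick.
; Meatiers spawns meteor warning actors at random XY positions on a delay, repeating while CurrentGame is "Meatiers".
; Obama Prism spawns one prism actor at a fixed spot and passes it a Harder flag.
; CurrentGame is never set in these graphs, and an unmatched pick prints an error and ends the cycle.
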(event `self.ReceiveBeginPlay`
  (switch `string` (`|GetArrayItem` (`self.games`) (`KismetMathLibrary.RandomIntegerInRange` 0 (- (`KismetArrayLibrary.Array_Length` (`self.games`)) 1))) :!label _label
    (:`Default`
      (`KismetSystemLibrary.PrintString` "Error, no minigame matching input was found"))
    (:`Meatiers`
      (`self.Meatiers` 0.5)
      (`KismetSystemLibrary.Delay` 6.0 :!label _label_2)
      (goto _label))
    (:`Obama Prism`
      (`self.Obama Prism` false)
      (goto _label_2))))

(event `Meatiers`
  (params (`meatier delay` :type "Float (double-precision)"))
  (`|SpawnActorFromClass` "/Game/blueprints/BP_meatier_warning.BP_meatier_warning_C" (`KismetMathLibrary.MakeTransform` (`KismetMathLibrary.MakeVector` (`KismetMathLibrary.RandomFloatInRange` 720.0 2280.0) (`KismetMathLibrary.RandomFloatInRange` 740.0 3040.0))) "Undefined" "MultiplyWithRoot" null null :!label _label_3)
  (`KismetSystemLibrary.Delay` `meatier delay`)
  (if (== (`self.current game`) "Meatiers")
    (goto _label_3)))

(event `Obama Prism`
  (params (harder :type Boolean))
  (bind _returnvalue (`|SpawnActorFromClass` "/Game/blueprints/BP_obama_prism.BP_obama_prism_C" (`KismetMathLibrary.MakeTransform` (1110.0 3240.0 -20.0)) "Undefined" "MultiplyWithRoot" null null))
  (set `/Game/blueprints/BP_obama_prism.harder` harder _returnvalue))

(fn `UserConstructionScript`)