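; BP_obama_prism is a self-destroying laser hazard that slides in, fires, then turns around and retreats.
; BeginPlay runs the timeline as a chain of MoveComponentTo and Delay nodes, toggling the laser's visibility and collision.
; The Harder flag makes it sweep the beam in yaw rather than hold still.
; A BP_TopDownCharacter overlapping the laser gets briefly stunned through its BP_PC_Lobby controller.
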(event `self.ReceiveBeginPlay`
  (bind _returnvalue (`self.GetTransform`))
  (bind _returnvalue_2 (`self.GetTransform`))
  (bind _returnvalue_3 (`self.GetTransform`))
  (bind _returnvalue_4 (`self.GetTransform`))
  (bind _returnvalue_5 (`self.GetTransform`))
  (bind _returnvalue_6 (`self.GetTransform`))
  (`PrimitiveComponent.SetCollisionEnabled` (`self.laser`) "NoCollision")
  (`self.K2_SetActorRotation` (struct :`Yaw` 90.0))
  (`KismetSystemLibrary.MoveComponentTo` (`self.DefaultSceneRoot`) (`KismetMathLibrary.MakeVector` (.x (.location _returnvalue_2)) (+ (.y (.location _returnvalue_2)) -500.0) (.z (.location _returnvalue_2))) (.rotation _returnvalue_2) true false 3.0)
  (if (`self.harder`)
    (`KismetSystemLibrary.MoveComponentTo` (`self.DefaultSceneRoot`) (.location _returnvalue_4) (`KismetMathLibrary.MakeRotator` 0.0 0.0 (+ (.yaw (.rotation _returnvalue_4)) -20.0)) true true 0.5))
  (`KismetSystemLibrary.Delay` 0.2)
  (`SceneComponent.SetVisibility` (`self.laser`) true false)
  (`PrimitiveComponent.SetCollisionEnabled` (`self.laser`) "QueryOnly")
  (if (`self.harder`)
    (`KismetSystemLibrary.MoveComponentTo` (`self.DefaultSceneRoot`) (.location _returnvalue_5) (`KismetMathLibrary.MakeRotator` 0.0 0.0 (+ (.yaw (.rotation _returnvalue_5)) 40.0)) true true 3.0)
    (`KismetSystemLibrary.Delay` 0.2)
    (`SceneComponent.SetVisibility` (`self.laser`) false false)
    (`PrimitiveComponent.SetCollisionEnabled` (`self.laser`) "NoCollision")
    (`KismetSystemLibrary.Delay` 0.1)
    (`KismetSystemLibrary.MoveComponentTo` (`self.DefaultSceneRoot`) (.location _returnvalue) (`KismetMathLibrary.MakeRotator` 0.0 0.0 (+ (.yaw (.rotation _returnvalue)) -20.0)) true true)
    (else
      (`KismetSystemLibrary.Delay` 3.0)))
  (`SceneComponent.SetVisibility` (`self.laser`) false false)
  (`PrimitiveComponent.SetCollisionEnabled` (`self.laser`) "NoCollision")
  (`KismetSystemLibrary.Delay` 0.2)
  (`KismetSystemLibrary.MoveComponentTo` (`self.DefaultSceneRoot`) (.location _returnvalue_3) (`KismetMathLibrary.MakeRotator` (.roll (.rotation _returnvalue_3)) (.pitch (.rotation _returnvalue_3)) (- (.yaw (.rotation _returnvalue_3)) 180.0)) true true 0.75)
  (`KismetSystemLibrary.MoveComponentTo` (`self.DefaultSceneRoot`) (`KismetMathLibrary.MakeVector` (.x (.location _returnvalue_6)) (+ (.y (.location _returnvalue_6)) 500.0) (.z (.location _returnvalue_6))) (.rotation _returnvalue_6) true true 0.75)
  (`self.K2_DestroyActor`))

(event `self.laser.OnComponentBeginOverlap`
  (params (OverlappedComponent :type "PrimitiveComponent Object Reference") (OtherActor :type "Actor Object Reference") (OtherComp :type "PrimitiveComponent Object Reference") (OtherBodyIndex :type Integer) (bFromSweep :type Boolean) (SweepResult :type "HitResult Structure (by ref)"))
  (if (== (`GameplayStatics.GetObjectClass` OtherActor) "/Game/TopDown/Blueprints/BP_TopDownCharacter.BP_TopDownCharacter_C")
    (bind _asbp_top_down_character (cast `/Game/TopDown/Blueprints/BP_TopDownCharacter` OtherActor))
    (bind _asbp_pc_lobby (cast `/Game/blueprints/lobby/BP_PC_Lobby` (`Pawn.GetController` _asbp_top_down_character)))
    (`/Game/blueprints/lobby/BP_PC_Lobby.stunned` _asbp_pc_lobby 0.7)))

(fn `UserConstructionScript`)