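; Falling meteor actor that crashes to the ground and briefly stuns any player it hits.
; On BeginPlay it stores its starting height, then each Tick counts a timer down and lerps its Z toward a fixed ground height, destroying itself when the timer runs out.
; Overlapping a BP_TopDownCharacter calls Stunned on that character's BP_PC_Lobby controller.
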(event `self.ReceiveBeginPlay`
  ;[1 1 1] Set starting values
  (set `self.timer` (`self.timer start`))
  (set `self.starting height` (.z (.location (`self.GetTransform`)))))

(event `self.ReceiveTick`
  (params (DeltaSeconds :type "Float (single-precision)"))
  (bind _returnvalue (`self.GetTransform`))
  ;[1 1 1] Make the meatier crash to the earth
  (bind _output_get (set `self.timer` (- (`self.timer`) DeltaSeconds)))
  (`self.K2_SetActorTransform` (`KismetMathLibrary.MakeTransform` (`KismetMathLibrary.MakeVector` (.x (.location _returnvalue)) (.y (.location _returnvalue)) (`KismetMathLibrary.Lerp` -49.0 (`self.starting height`) (`KismetMathLibrary.SafeDivide` _output_get (`self.timer start`)))) (.rotation _returnvalue) (.scale _returnvalue)))
  (if (<= (`self.timer`) 0.0)
    (`self.K2_DestroyActor`)))

(event `self.ReceiveActorBeginOverlap`
  (params (OtherActor :type "Actor Object Reference"))
  ;[1 1 1] Stun hit players
  (if (== (`GameplayStatics.GetObjectClass` OtherActor) "/Game/TopDown/Blueprints/BP_TopDownCharacter.BP_TopDownCharacter_C")
    (bind _asbp_top_down_character (cast `/Game/TopDown/Blueprints/BP_TopDownCharacter` OtherActor))
    (bind _asbp_pc_lobby (cast `/Game/blueprints/lobby/BP_PC_Lobby` (`Pawn.GetController` _asbp_top_down_character)))
    (`/Game/blueprints/lobby/BP_PC_Lobby.stunned` _asbp_pc_lobby 0.7)))

(fn `UserConstructionScript`)